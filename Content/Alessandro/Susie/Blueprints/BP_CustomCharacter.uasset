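; Player character with walk/run toggle, gun drawing, jello bouncing and NPC talk, exposing movement and action functions as delegates.
; It spawns a sheathed gun, and aiming functions switch rotation modes while a timeline slides the camera.
; Bounce-tagged hits launch it along the impact normal and animate a material parameter collection.
; Input swaps possession to a height-map pawn, while catapult overlap blends to its camera and moves it.
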(event `self.ReceiveBeginPlay`
  (`self.GenerateGun`)
  (bind _returnvalue (`GameplayStatics.GetActorOfClass` "/Game/Alessandro/BP_HeightMapPawn.BP_HeightMapPawn_C"))
  (`/Engine/EditorBlueprintResources/StandardMacros.IsValid` _returnvalue
    (:`Is Valid`
      (set `self.HighMapView_ref` _returnvalue)
      (bind _returnvalue_2 (`GameplayStatics.GetActorOfClass` "/Game/Alessandro/Catapulta/BP_Catapulta.BP_Catapulta_C"))
      (set `self.CatapultRef` _returnvalue_2)
      (bind _returnvalue_3 (`GameplayStatics.GetActorOfClass` "/Game/Alessandro/BP_CatapultViewCamera.BP_CatapultViewCamera_C"))
      (set `self.catapultViewRef` _returnvalue_3))))

(event `MoveCameraForward`
  (bind _followcamera (`self.FollowCamera`))
  (bind (_relativelocation_x _relativelocation_y _relativelocation_z) (`KismetMathLibrary.BreakVector` (`SceneComponent.RelativeLocation` _followcamera)))
  ;[1 1 1] Custom event that handles camera movements forward/backwards when aiming
  (bind (_direction _moving) (`Timeline|Timeline` :!label _label)
    (:`Update`
      (`SceneComponent.K2_SetRelativeLocation` _followcamera (`KismetMathLibrary.MakeVector` (* _moving (`self.cameraXoffset`)) _relativelocation_y _relativelocation_z) false false))))

(event `MoveCameraBackwards`
  ;[1 1 1] Custom event that handles camera movements forward/backwards when aiming
  (goto _label :!via `ReverseFromEnd`))

(event `self.CapsuleComponent.OnComponentHit`
  (params (HitComponent :type "PrimitiveComponent Object Reference") (OtherActor :type "Actor Object Reference") (OtherComp :type "PrimitiveComponent Object Reference") (NormalImpulse :type "Vector Structure") (Hit :type "HitResult Structure (by ref)"))
  (bind (_bblockinghit _binitialoverlap _time _distance _location _impactpoint _normal _impactnormal _physmat _hitactor _hitcomponent) (`GameplayStatics.BreakHitResult` Hit))
  ;[1 1 1] Custom event for jumping logic on jellos
  (if (`ActorComponent.ComponentHasTag` _hitcomponent "Bounce")
    (`KismetSystemLibrary.Delay` 0.1)
    (`self.LaunchCharacter` self (* _impactnormal (`self.LaunchStregth`)) false false)
    (`KismetMaterialLibrary.SetVectorParameterValue` "/Game/Alessandro/Jello/MPC_BounceData.MPC_BounceData" "Location" (`KismetMathLibrary.Conv_VectorToLinearColor` _impactpoint))
    (bind (_direction _buonce_values) (`Timeline|Timeline_1` :!via `PlayFromStart`)
      (:`Update`
        (`KismetMaterialLibrary.SetVectorParameterValue` "/Game/Alessandro/Jello/MPC_BounceData.MPC_BounceData" "Normal" (`KismetMathLibrary.Conv_VectorToLinearColor` (* _impactnormal (* _buonce_values (`self.BounceIntensity`)))))))))

(event `EnhancedInput|/Game/ThirdPerson/Input/Actions/IA_SwitchView`
  (params (ActionValue :type Boolean) (ElapsedSeconds :type "Float (double-precision)") (TriggeredSeconds :type "Float (double-precision)") (InputAction :type "InputAction Object Reference" :default "/Game/ThirdPerson/Input/Actions/IA_SwitchView.IA_SwitchView"))
  (:`Started`
    (`self.SwitchToMapView`)))

(event `self.CapsuleComponent.OnComponentBeginOverlap`
  (params (OverlappedComponent :type "PrimitiveComponent Object Reference") (OtherActor :type "Actor Object Reference") (OtherComp :type "PrimitiveComponent Object Reference") (OtherBodyIndex :type Integer) (bFromSweep :type Boolean) (SweepResult :type "HitResult Structure (by ref)"))
  (cast `/Game/Alessandro/Catapulta/BP_Catapulta` OtherActor
    (:`then`
      (`self.SetCameraViewForCatapult`))
    (:`CastFailed`
      (bind _asbp_generic_npc (cast `/Game/Alessandro/NPC/BP_GenericNPC` OtherActor))
      (set `self.currentNPCref` _asbp_generic_npc))))

(event `EnhancedInput|/Game/ThirdPerson/Input/Actions/IA_Interact`
  (params (ActionValue :type Boolean) (ElapsedSeconds :type "Float (double-precision)") (TriggeredSeconds :type "Float (double-precision)") (InputAction :type "InputAction Object Reference" :default "/Game/ThirdPerson/Input/Actions/IA_Interact.IA_Interact"))
  (:`Started`
    (bind _currentnpcref (`self.currentNPCref`)
      (:`then`
        (`/Game/Alessandro/NPC/BP_GenericNPC.Talk` _currentnpcref))
      (:`else`))))

(fn `Change Character Orientation for Walking`
  (`self.MoveCameraBackwards`)
  (set `CharacterMovementComponent.bOrientRotationToMovement` true (`self.CharacterMovement`))
  (set `self.bUseControllerRotationYaw` false)
  (set `self.bUseControllerRotationPitch` false)
  (set `SpringArmComponent.bUsePawnControlRotation` true (`self.SpringArm`)))

(fn `ChangeCharacterOrientationForAiming`
  (`self.MoveCameraForward`)
  (set `CharacterMovementComponent.bOrientRotationToMovement` false (`self.CharacterMovement`))
  (set `self.bUseControllerRotationYaw` true)
  (set `self.bUseControllerRotationPitch` true)
  (set `SpringArmComponent.bUsePawnControlRotation` false (`self.SpringArm`)))

(fn `Draw Stash Delegate`
  (returns (animDuration :type "Float (double-precision)"))
  (if (`self.isGunEquipped?`)
    (bind _returnvalue (`self.PlayAnimMontage` "/Game/Alessandro/Susie/Animations/AM_Stashing_Gun_Montage.AM_Stashing_Gun_Montage"))
    (return _returnvalue)
    (else
      (bind _returnvalue_2 (`self.PlayAnimMontage` "/Game/Alessandro/Susie/Animations/AM_Drawing_Gun.AM_Drawing_Gun"))
      (return _returnvalue_2))))

(fn `GenerateGun`
  (bind _returnvalue (`|SpawnActorFromClass` "/Game/Alessandro/Gun/BP_Gun.BP_Gun_C" (`SceneComponent.GetSocketTransform` (`self.Mesh`) "Sheath" "RTS_World") "AdjustIfPossibleButAlwaysSpawn" "MultiplyWithRoot" null null))
  (bind _output_get (set `self.gunREF` _returnvalue))
  (`self.K2_AttachToComponent` _output_get (`self.Mesh`) "Sheath" "SnapToTarget" "SnapToTarget" "SnapToTarget" true))

(fn `Look Delegate`
  (params (x :type "Float (double-precision)") (y :type "Float (double-precision)"))
  (`self.AddControllerYawInput` x)
  (`self.AddControllerPitchInput` y))

(fn `MoveDelegate`
  (params (x :type "Float (double-precision)") (y :type "Float (double-precision)"))
  (bind (_returnvalue_roll _returnvalue_pitch _returnvalue_yaw) (`KismetMathLibrary.BreakRotator` (`self.GetControlRotation`)))
  (bind (_returnvalue_roll_2 _returnvalue_pitch_2 _returnvalue_yaw_2) (`KismetMathLibrary.BreakRotator` (`self.GetControlRotation`)))
  (`self.AddMovementInput` (`KismetMathLibrary.GetRightVector` (`KismetMathLibrary.MakeRotator` _returnvalue_roll_2 0.0 _returnvalue_yaw_2)) x)
  (`self.AddMovementInput` (`KismetMathLibrary.GetForwardVector` (`KismetMathLibrary.MakeRotator` 0.0 0.0 _returnvalue_yaw)) (* y 1.0)))

(fn `RunDelegate`
  (bind _charactermovement (`self.CharacterMovement`))
  (if (`self.isRunning?`)
    (set `CharacterMovementComponent.MaxWalkSpeed` (`self.walkingSpeed`) _charactermovement)
    (set `self.isRunning?` false)
    (else
      (set `CharacterMovementComponent.MaxWalkSpeed` (`self.runningSpeed`) _charactermovement)
      (set `self.isRunning?` true))))

(fn `SetCameraViewForCatapult`
  (`PlayerController.SetViewTargetWithBlend` (`GameplayStatics.GetPlayerController` 0) (`self.catapultViewRef`) 0.0 "VTBlend_Linear" 0.0 false)
  (`/Game/Alessandro/Catapulta/BP_Catapulta.MoveCatapult` (`self.CatapultRef`)))

(fn `SwitchToMapView`
  (bind _returnvalue (`GameplayStatics.GetPlayerController` 0))
  (`Controller.UnPossess` _returnvalue)
  (`Controller.Possess` _returnvalue (`self.HighMapView_ref`))
  (bind _asbpc_custom_controller (cast `/Game/Alessandro/Susie/Blueprints/BPC_CustomController` _returnvalue))
  (bind _returnvalue_2 (pcsubsystem `EnhancedInputLocalPlayerSubsystem` _asbpc_custom_controller))
  (`EnhancedInputSubsystemInterface.RemoveMappingContext` _returnvalue_2 "/Game/ThirdPerson/Input/IMC_Default.IMC_Default" (struct))
  (`EnhancedInputSubsystemInterface.AddMappingContext` _returnvalue_2 "/Game/ThirdPerson/Input/IMC_MapMovements.IMC_MapMovements" 0 (struct)))

(fn `UserConstructionScript`)