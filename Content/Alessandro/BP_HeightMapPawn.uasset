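; BP_HeightMapPawn is a map-view pawn that gives the player a rotatable, zoomable spring-arm camera as an alternative to the character view.
; Enhanced Input actions yaw the controlled pawn and change the arm length, scaled by delta time, with no zoom clamp.
; At BeginPlay it caches the controlled BP_CustomCharacter.
; The switch-view input possesses that character again and swaps IMC_MapMovements for IMC_Default.
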(event `self.ReceiveBeginPlay`
  (`self.GetReferenceToCharacter`))

(event `EnhancedInput|/Game/ThirdPerson/Input/Actions/IA_SwitchView`
  (params (ActionValue :type Boolean) (ElapsedSeconds :type "Float (double-precision)") (TriggeredSeconds :type "Float (double-precision)") (InputAction :type "InputAction Object Reference" :default "/Game/ThirdPerson/Input/Actions/IA_SwitchView.IA_SwitchView"))
  ;[0 0.08547 1] MAP INPUTS
  ;;[1 1 1] Switch view
  (:`Started`
    (`self.SwitchToCharacterView`)))

(event `EnhancedInput|/Game/ThirdPerson/Input/Actions/IA_RotateMap`
  (params (ActionValue :type "Float (double-precision)") (ElapsedSeconds :type "Float (double-precision)") (TriggeredSeconds :type "Float (double-precision)") (InputAction :type "InputAction Object Reference" :default "/Game/ThirdPerson/Input/Actions/IA_RotateMap.IA_RotateMap"))
  ;[0 0.08547 1] MAP INPUTS
  ;;[1 1 1] Rotation
  (:`Triggered`
    (bind _asbpc_custom_controller (cast `/Game/Alessandro/Susie/Blueprints/BPC_CustomController` (`GameplayStatics.GetPlayerController` 0)))
    (`self.K2_AddActorWorldRotation` (`Controller.K2_GetPawn` _asbpc_custom_controller) (`KismetMathLibrary.MakeRotator` 0.0 0.0 (* ActionValue (`self.CameraRotiationSpeed`) (`GameplayStatics.GetWorldDeltaSeconds`))) false false)))

(event `EnhancedInput|/Game/ThirdPerson/Input/Actions/IA_ZoomMap`
  (params (ActionValue :type "Float (double-precision)") (ElapsedSeconds :type "Float (double-precision)") (TriggeredSeconds :type "Float (double-precision)") (InputAction :type "InputAction Object Reference" :default "/Game/ThirdPerson/Input/Actions/IA_ZoomMap.IA_ZoomMap"))
  (bind _springarm (`self.SpringArm`))
  ;[0 0.08547 1] MAP INPUTS
  ;;[1 1 1] Zoom in/out
  (:`Triggered`
    (set `SpringArmComponent.TargetArmLength` (+ (`SpringArmComponent.TargetArmLength` _springarm) (* (* ActionValue (`self.zoomOffset`)) (`GameplayStatics.GetWorldDeltaSeconds`))) _springarm)))

(fn `GetReferenceToCharacter`
  (returns (Controller :type "PlayerController Object Reference"))
  (bind _returnvalue (`GameplayStatics.GetPlayerController` 0))
  (bind _asbp_custom_character (cast `/Game/Alessandro/Susie/Blueprints/BP_CustomCharacter` (`Controller.K2_GetPawn` _returnvalue))
    (:`then`
      (set `self.characterRef` _asbp_custom_character))
    (:`CastFailed`
      (`KismetSystemLibrary.PrintString` "CAST CHARACTER FALLITO")))
  (return _returnvalue))

(fn `SwitchToCharacterView`
  (bind _returnvalue (`GameplayStatics.GetPlayerController` 0))
  (`Controller.UnPossess` _returnvalue)
  (`Controller.Possess` _returnvalue (`self.characterRef`))
  (bind _asbpc_custom_controller (cast `/Game/Alessandro/Susie/Blueprints/BPC_CustomController` _returnvalue))
  (bind _returnvalue_2 (pcsubsystem `EnhancedInputLocalPlayerSubsystem` _asbpc_custom_controller))
  (message `EnhancedInputSubsystemInterface.RemoveMappingContext` _returnvalue_2 "/Game/ThirdPerson/Input/IMC_MapMovements.IMC_MapMovements" (struct))
  (message `EnhancedInputSubsystemInterface.AddMappingContext` _returnvalue_2 "/Game/ThirdPerson/Input/IMC_Default.IMC_Default" 0 (struct)))

(fn `UserConstructionScript`
  (bind _springarm (`self.SpringArm`))
  (set `SpringArmComponent.TargetOffset` (0.0 0.0 0.0) _springarm)
  (set `SpringArmComponent.TargetArmLength` (`self.armLenghtDistanceOffset`) _springarm))