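; BP_Catapulta is a catapult that launches the player's BP_CustomCharacter.
; On BeginPlay it caches the player's controlled character.
; MoveCatapult plays the Positioning timeline to roll RotationPoint by a scaled offset, then launches that character along the Arrow component's forward vector with an added upward boost.
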(event `self.ReceiveBeginPlay`
  (bind _asbp_custom_character (cast `/Game/Alessandro/Susie/Blueprints/BP_CustomCharacter` (`Controller.K2_GetPawn` (`GameplayStatics.GetPlayerController` 0))))
  (set `self.characterRef` _asbp_custom_character))

(event `MoveCatapult`
  (bind (_direction _initialmovement) (`Timeline|Positioning` :!via `PlayFromStart`)
    (:`Update`
      (`SceneComponent.K2_SetRelativeRotation` (`self.RotationPoint`) (`KismetMathLibrary.MakeRotator` (* _initialmovement (`self.InitialPositioningOffset`))) false false))
    (:`Finished`
      (bind _characterref (`self.characterRef`)
        (:`then`
          (`Character.LaunchCharacter` _characterref (+ (* (`SceneComponent.GetForwardVector` (`self.Arrow`)) 2000.0) (0.0 0.0 500.0)) false false))
        (:`else`)))))

(fn `UserConstructionScript`)