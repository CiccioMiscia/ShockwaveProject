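; Generic talkable NPC Blueprint that shows an interaction prompt and steps through dialogue lines when the player is nearby.
; Entering the trigger area creates the prompt and dialogue widgets, and leaving removes them and resets the conversation.
; Each Talk call shows the next SpeechData line, using a resettable DoOnce to add the dialogue box once per conversation, and closes it after the last line.
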(event `self.TriggerArea.OnComponentBeginOverlap`
  (params (OverlappedComponent :type "PrimitiveComponent Object Reference") (OtherActor :type "Actor Object Reference") (OtherComp :type "PrimitiveComponent Object Reference") (OtherBodyIndex :type Integer) (bFromSweep :type Boolean) (SweepResult :type "HitResult Structure (by ref)"))
  (bind _returnvalue (`GameplayStatics.GetPlayerController` 0))
  (if (== OtherActor (`GameplayStatics.GetPlayerCharacter` 0))
    (bind _returnvalue_2 (`|CreateWidget` "/Game/Alessandro/NPC/WBP_InteractionText.WBP_InteractionText_C" _returnvalue))
    (bind _output_get (set `self.UI_Interaction` _returnvalue_2))
    (`UserWidget.AddToViewport` _output_get 0)
    (bind _returnvalue_3 (`|CreateWidget` "/Game/Alessandro/NPC/WBP_DialogueText.WBP_DialogueText_C" _returnvalue))
    (bind _output_get_2 (set `self.UI_Dialogue` _returnvalue_3))
    (`TextBlock.SetText` (`/Game/Alessandro/NPC/WBP_DialogueText.Name` _output_get_2) (`self.Name`))))

(event `self.TriggerArea.OnComponentEndOverlap`
  (params (OverlappedComponent :type "PrimitiveComponent Object Reference") (OtherActor :type "Actor Object Reference") (OtherComp :type "PrimitiveComponent Object Reference") (OtherBodyIndex :type Integer))
  (`Widget.RemoveFromParent` (`self.UI_Interaction`))
  (bind _ui_dialogue (`self.UI_Dialogue`)
    (:`then`
      (`Widget.RemoveFromParent` _ui_dialogue)
      (set `self.lineIndex` 0)
      (`self.ResetDialogue`))
    (:`else`)))

(event `Talk`
  (bind _speechdata (`self.SpeechData`))
  (bind _lineindex (`self.lineIndex`))
  (bind _ui_dialogue (`self.UI_Dialogue`)
    (:`then`
      (`|ExecutionSequence`
        (:`then_0`
          (`/Engine/EditorBlueprintResources/StandardMacros.DoOnce` false :!label _label
            (:`Completed`
              (`UserWidget.AddToViewport` _ui_dialogue 0))))
        (:`then_1`
          (if (< _lineindex (`KismetArrayLibrary.Array_Length` _speechdata))
            (`TextBlock.SetText` (`/Game/Alessandro/NPC/WBP_DialogueText.speech` (`self.UI_Dialogue`)) (`KismetTextLibrary.Conv_StringToText` (`.Line_9_BA865FD749B98052221848BC0FFB9FA5` (break `/Game/Alessandro/NPC/S_DialogueData` (`|GetArrayItem` _speechdata _lineindex)))))
            (`/Engine/EditorBlueprintResources/StandardMacros.IncrementInt` (`self.lineIndex`))
            (else
              (`Widget.RemoveFromParent` (`self.UI_Dialogue`))
              (set `self.lineIndex` 0)
              (`self.ResetDialogue`))))))
    (:`else`)))

(event `ResetDialogue`
  (goto _label :!via `Reset`))

(fn `UserConstructionScript`)