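; BP_Croissant is a croissant actor built to roll back and forth, with an overlap box intended for destroying jellos.
; Paired timelines drive mesh roll and relative X movement, each looping forward and reverse, but nothing connected starts them.
; On overlap, it checks its own box for the CroissantDestroyable tag, prints debug text and, if tagged, destroys itself rather than the other actor.
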(event `self.ReceiveBeginPlay`)

(event `self.ReceiveTick`
  (params (DeltaSeconds :type "Float (single-precision)")))

(event `RotateRoller`
  ;[1 1 1] CROISSANT ROTATIONS
  ;;[1 1 1] Function for rotating 0 - 360
  (bind (_direction _rotation) (`Timeline|Rotation` :!via `PlayFromStart`)
    (:`Update`
      (`SceneComponent.K2_AddRelativeRotation` (`self.StaticMesh`) (`KismetMathLibrary.MakeRotator` (* _rotation (`self.RotationVelocity`))) false false))
    (:`Finished`
      (`self.ReverseRotateRoller`))))

(event `MoveRoller`
  (bind (_returnvalue_x _returnvalue_y _returnvalue_z) (`KismetMathLibrary.BreakVector` (`SceneComponent.GetForwardVector` (`self.MovementDirection`))))
  ;[1 1 1] CROISSANT MOVEMENT
  ;;[1 1 1] Function for moving Croissant towards a direction
  (bind (_direction _movements) (`Timeline|Movement` :!via `PlayFromStart`)
    (:`Update`
      (`SceneComponent.K2_SetRelativeLocation` (`self.StaticMesh`) (`KismetMathLibrary.MakeVector` (+ (* _movements (`self.MovementSpeed`)) _returnvalue_x) _returnvalue_y _returnvalue_z) false false))
    (:`Finished`
      (`self.ReverseRoller`))))

(event `ReverseRotateRoller`
  ;[1 1 1] CROISSANT ROTATIONS
  ;;[1 1 1] Function to rotate 360-0
  (bind (_direction _rotation) (`Timeline|Rotation_2` :!via `ReverseFromEnd`)
    (:`Update`
      (`SceneComponent.K2_AddRelativeRotation` (`self.StaticMesh`) (`KismetMathLibrary.MakeRotator` (* _rotation (`self.RotationVelocity`))) false false))
    (:`Finished`
      (`self.RotateRoller`))))

(event `ReverseRoller`
  ;[1 1 1] CROISSANT MOVEMENT
  ;;[1 1 1] Function for getting back the Croissant
  (bind (_direction _movements) (`Timeline|Timeline` :!via `ReverseFromEnd`)
    (:`Update`
      (bind _returnvalue_x (`KismetMathLibrary.BreakVector` (+ (* _movements (`self.MovementSpeed`)) (`SceneComponent.GetForwardVector` (`self.MovementDirection`)))))
      (`SceneComponent.K2_SetRelativeLocation` (`self.StaticMesh`) (`KismetMathLibrary.MakeVector` _returnvalue_x) false false))
    (:`Finished`
      (`self.MoveRoller`))))

(event `self.Box.OnComponentBeginOverlap`
  (params (OverlappedComponent :type "PrimitiveComponent Object Reference") (OtherActor :type "Actor Object Reference") (OtherComp :type "PrimitiveComponent Object Reference") (OtherBodyIndex :type Integer) (bFromSweep :type Boolean) (SweepResult :type "HitResult Structure (by ref)"))
  ;[1 1 1] Function for destroying Jellos if hit by Croissants
  (if (`ActorComponent.ComponentHasTag` OverlappedComponent "CroissantDestroyable")
    (`KismetSystemLibrary.PrintString` "COLPISCO GELATINA")
    (`self.K2_DestroyActor`)
    (else
      (`KismetSystemLibrary.PrintString` "NON COLPISCO GELATINA"))))

(fn `UserConstructionScript`)